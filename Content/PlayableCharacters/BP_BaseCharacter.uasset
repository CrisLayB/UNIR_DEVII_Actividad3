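; Base playable character Blueprint holding a Stats struct with HP, MP, ATB and name.
; GetDamage subtracts damage from current HP, floors it at zero and writes it back to Stats.
; Its return value re-evaluates that subtraction on the updated HP, so damage counts twice there.
; On landing, a living character clears the mesh's physics blend weight to exit ragdoll, relying on a disabled pelvis bone to avoid repositioning.
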(event `self.OnLanded`
  (params (Hit :type "HitResult Structure (by ref)"))
  (bind _stats_currenthp (break `/Game/PlayableCharacters/S_CharacterStats` (`self.Stats`)))
  ; If we've landed and are still alive, reset ragdoll physics so we can resume gameplay. Since we disabled the pelvis bone, we don't need to reset the mesh to its original location.
  (if (> _stats_currenthp 0.0)
    (`SkeletalMeshComponent.SetPhysicsBlendWeight` (`self.Mesh`) 0.0)))

(fn `GetDamage`
  (params (damage :type "Float (double-precision)"))
  (returns (newDamage :type "Float (double-precision)"))
  (bind _stats_currenthp (break `/Game/PlayableCharacters/S_CharacterStats` (`self.Stats`)))
  (bind (_stats_currenthp_2 _stats_maxhp _stats_currentmp _stats_maxmp _stats_currentatb _stats_maxatb _stats_charactername) (break `/Game/PlayableCharacters/S_CharacterStats` (`self.Stats`)))
  (bind _returnvalue (- _stats_currenthp damage))
  (bind _returnvalue_2 (select `bool` (<= _returnvalue 0.0) :`false` _returnvalue))
  (set `self.Stats` (make `/Game/PlayableCharacters/S_CharacterStats` _returnvalue_2 _stats_maxhp _stats_currentmp _stats_maxmp _stats_currentatb _stats_maxatb _stats_charactername))
  (return _returnvalue_2))

(fn `UserConstructionScript`)